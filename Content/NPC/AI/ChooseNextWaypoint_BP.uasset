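; Behavior tree task that selects the next patrol waypoint for an AI-controlled NPC.
; On execute, it casts the controlled pawn and copies its patrol point array.
; It writes the point at the blackboard index to the Waypoint key, then increments that index with modulo wraparound so the route loops.
; The task then finishes with success, though a failed cast leaves the point array unset.
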(event `self.ReceiveExecuteAI`
  (params (OwnerController :type "AIController Object Reference") (ControlledPawn :type "Pawn Object Reference"))
  (`self.Get patrol points` ControlledPawn)
  (`self.Cycle inde`)
  (`self.FinishExecute` true))

(fn `Cycle inde`
  (bind _index (`self.Set nextway point`))
  (`BTFunctionLibrary.SetBlackboardValueAsInt` (`self.index`) (mod (+ _index 1) (`KismetArrayLibrary.Array_Length` (`self.patrol points`)))))

(fn `Get patrol points`
  (params (Object :type "Object Object Reference"))
  (bind _asthird_person_character (cast `` Object))
  (set `self.patrol points` (`/Game/NPC/AI/ChooseNextWaypoint_BP.Patrol_points` _asthird_person_character)))

(fn `Set nextway point`
  (returns (index :type Integer))
  (bind _returnvalue (`BTFunctionLibrary.GetBlackboardValueAsInt` (`self.index`)))
  (`BTFunctionLibrary.SetBlackboardValueAsObject` (`self.Waypoint`) (`|GetArrayItem` (`self.patrol points`) _returnvalue))
  (return _returnvalue))