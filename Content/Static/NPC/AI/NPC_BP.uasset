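; NPC AI controller that runs a guard behavior tree on patrol blackboard data and tracks an enemy through AI perception.
; On BeginPlay it initializes the blackboard and starts the tree.
; Perception updates for actors tagged "Enemy" write the enemy key.
; Successful sensing clears that key, while lost sensing sets it to player pawn 0 rather than the perceived actor.
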(event `self.ReceiveBeginPlay`
  (bind _blackboardcomponent (`self.UseBlackboard` "/Game/Static/NPC/AI/PatolData.PatolData"))
  (`self.RunBehaviorTree` "/Game/Static/NPC/AI/GuardBehaviour.GuardBehaviour")
  (set `self.Blackboardcomp` _blackboardcomponent))

(event `self.AIPerception.OnTargetPerceptionUpdated`
  (params (Actor :type "Actor Object Reference") (Stimulus :type "AIStimulus Structure"))
  (`self.Update blackboard enemy` Stimulus Actor))

(fn `Update blackboard enemy`
  (params (AIStimulus :type "AIStimulus Structure (by ref)") (self2 :type "Actor Object Reference"))
  (bind _enemey_key (`self.Enemey_Key`))
  (bind _blackboardcomp (`self.Blackboardcomp`))
  (if (`self.ActorHasTag` self2 "Enemy")
    (if (`.bSuccessfullySensed` (break `AIStimulus` AIStimulus))
      (`BlackboardComponent.ClearValue` _blackboardcomp _enemey_key)
      (else
        (`BlackboardComponent.SetValueAsObject` _blackboardcomp _enemey_key (`GameplayStatics.GetPlayerPawn` 0))))))

(fn `UserConstructionScript`)